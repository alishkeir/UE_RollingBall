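; Gear pickup Blueprint that spins in place and supplies its own point value, collect sound and gold sparkle effect.
; BeginPlay sets these pickup variables before calling the parent's BeginPlay.
; Tick adds a fixed world rotation each frame, so spin speed depends on frame rate.
; The overlap event is a disabled stub and the construction script only calls the parent, so this graph holds no collection logic.
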(event `self.ReceiveBeginPlay`
  (set `self.Points` 2)
  (set `self.PickupSound` "/Game/Retro_8Bit_Sounds/Collectables/Cues/retro_collect_pickup_coin_10_Cue.retro_collect_pickup_coin_10_Cue")
  (set `self.PickupParticles` "/Game/InfinityBladeEffects/Effects/FX_Treasure/Gold_Bag/P_GoldSparkle_Bag_Lo_2.P_GoldSparkle_Bag_Lo_2")
  (`parent.ReceiveBeginPlay`))

(event `self.ReceiveTick`
  (params (DeltaSeconds :type "Float (single-precision)"))
  (`parent.ReceiveTick` DeltaSeconds)
  (`self.K2_AddActorWorldRotation` (struct :`Yaw` 0.5)))

(fn `UserConstructionScript`
  (`parent.UserConstructionScript`))